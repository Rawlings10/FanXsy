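; BP_ProjectilePushDoor is an actor whose mesh gets knocked forward when hit by a projectile, as a pushable door.
; Its Box trigger responds only when the overlapping component is the BoxCollision of a BP_Projecctile_Base.
; A valid hit applies a mass-independent impulse along the mesh's forward vector, regardless of projectile direction.
; It also plays a falling-bricks sound at the actor and calls MakeNoise.
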(event OnComponentBeginOverlap(Box)
  (params (OverlappedComponent :type Primitive%20Component%20Object%20Reference) (OtherActor :type Actor%20Object%20Reference) (OtherComp :type Primitive%20Component%20Object%20Reference) (OtherBodyIndex :type Integer) (bFromSweep :type Boolean) (SweepResult :type Hit%20Result%20Structure%20%28by%20ref%29))
  (bind _asbp_projecctile_base (Utilities|Casting|CastToBP_Projecctile_Base OtherActor))
  (if (== (Variables|/Game/Projectiles/BP_Projecctile_Base.BP_Projecctile_Base_C|GetBox%20collision _asbp_projecctile_base) OtherComp)
    (Physics|AddImpulse (Variables|Default|GetStaticMesh) (* (Math|Vector|GetForwardVector (Variables|Default|GetStaticMesh)) 5e+03) "None" true)
    (Audio|PlaySoundatLocation "/Game/Sound/Sound_Cue/big-bricks-falling-sound-38428.big-bricks-falling-sound-38428" (Transformation|GetActorLocation) "0, 0, 0" 1.0 1.0 0.0 0 0 0 0)
    (Class|Actor|MakeNoise 1.0 0 "0, 0, 0" 0.0 "None")))

(event EventBeginPlay)

(event Collision|EventActorBeginOverlap
  (params (OtherActor :type Actor%20Object%20Reference)))

(event EventTick
  (params (DeltaSeconds :type Float%20%28single-precision%29)))

(fn ConstructionScript)