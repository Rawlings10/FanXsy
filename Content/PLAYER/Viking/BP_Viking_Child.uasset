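; BP_Viking_Child is a Viking player Blueprint that supplies the power values for its punch and kick attacks.
; Punch and Kick each read the hardcoded "Rob" row of DT_PlayersAbility and return PunchPower and KickPower respectively.
; BeginPlay and the construction script only call the parent versions, and neither lookup handles a missing row.
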(event EventBeginPlay
  (|CallParentFunction))

(event Collision|EventActorBeginOverlap
  (params (OtherActor :type Actor%20Object%20Reference)))

(event EventTick
  (params (DeltaSeconds :type Float%20%28single-precision%29)))

(fn ConstructionScript
  (|CallParentFunction))

(fn Punch
  (bind _returnvalue (Utilities|GetDataTableRow "/Game/PLAYER/ALL_PLAYERS/DT_PlayersAbility.DT_PlayersAbility" "Rob")
    (:then
      (return (.PunchPower (Utilities|Struct|BreakST_PlayerAbility _returnvalue))))))

(fn Kick
  (bind _returnvalue (Utilities|GetDataTableRow "/Game/PLAYER/ALL_PLAYERS/DT_PlayersAbility.DT_PlayersAbility" "Rob")
    (:then
      (return (.KickPower (Utilities|Struct|BreakST_PlayerAbility _returnvalue))))))