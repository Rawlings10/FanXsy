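; Actor component that handles health, healing and damage, including death, blocking and invincibility.
; TakeDamage reads a damage info struct and uses the CanBeDamge macro to route each hit to block, damage or no damage.
; Event dispatchers report blocks with their parry flag, death, and damage responses when the owner is interruptible or interruption is forced.
; Heal adds health clamped to the maximum while alive.
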(event EventBeginPlay)

(event EventTick
  (params (DeltaSeconds :type Float%20%28single-precision%29)))

(fn Heal
  (params (Amount :type Float%20%28double-precision%29))
  ;[0.15 0.15 0.15 0.5] Healing function takes the heal amount and add to current health and return the new health
  (if (not (Variables|Default|GetIsDead))
    (bind _output_get (Variables|Default|SetHealth (Math|Float|Clamp(Float) (+ Amount (Variables|Default|GetHealth)) 0.0 (Variables|Default|GetMaxHealth))))
    (return _output_get)))

(fn TakeDamage
  (params (DamageInfo :type ST%20Damage%20Info%20Structure))
  (bind (_amount _damagetype _damageresponse _damageinvincible _canbeblocked _canbeparried _shouldforceinterupt) (Utilities|Struct|BreakST_DamageInfo DamageInfo))
  ;[0.15 0.15 0.15 0.5] damage system (details more in the macro)
  (Utilities|CanbeDamge _damageinvincible _canbeblocked
    (:BlockDamge
      (Default|CallOnBlocked _canbeparried)
      (Development|PrintString "BLocked")
      (return false))
    (:DoDamage
      (bind _output_get (Variables|Default|SetHealth (- (Variables|Default|GetHealth) _amount)))
      (if (<= _output_get 0.0)
        (Variables|Default|SetIsDead true)
        (Development|PrintString "Dead")
        (Default|CallOnDealth)
        (Development|PrintString "Damage" :!label _label)
        (return true)
        (elif (or (Variables|Default|GetIsInterruptible) _shouldforceinterupt)
          (Default|CallOnDamageResponse _damageresponse)
          (goto _label))))
    (:NoDamage
      (Development|PrintString "No Damage")
      (return false))))