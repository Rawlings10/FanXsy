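; Melee enemy Blueprint that draws, swings and sheathes a sword, with each action driven by a montage and its notify.
; Equip spawns BP_Sword onto the SK_Sword socket; unequip destroys it.
; Attack sphere-traces forward for pawns, sends damage read from DT_DamagePower, and disables damage-system interruptibility until the montage ends.
; Completion dispatchers report back, though the equipped and unequipped calls are swapped.
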(event EventUnequipWeapon
  ;[0.15 0.15 0.15 0.5] Wierd sword
  (bind _notifyname (Animation|Montage|PlayMontage (Variables|Character|GetMesh) "/Game/ENEMY/animation/montage/Sheathing_Sword_Montage.Sheathing_Sword_Montage")
    (:OnCompleted
      (Default|CallOnWeaponEquiped))
    (:OnNotifyBegin
      (switch name _notifyname
        (:Drop%20Sword
          (Actor|DestroyActor (Variables|Default|GetWeapon))
          (Variables|Default|SetisWieldingWeapon false))))))

(event EventEquipWeapon
  ;[0.15 0.15 0.15 0.5] enemy wield sword
  (bind _notifyname (Animation|Montage|PlayMontage (Variables|Character|GetMesh) "/Game/ENEMY/animation/montage/Weirlding_Sword_Montage1.Weirlding_Sword_Montage1")
    (:OnCompleted
      (Default|CallOnWeaponUnEquiped))
    (:OnNotifyBegin
      (switch name _notifyname
        (:Open%20Sword
          (bind _returnvalue (Game|SpawnActorfromClass "/Game/Weapons/BP_Sword.BP_Sword_C" (Transformation|GetActorTransform) "Undefined" "MultiplyWithRoot" 0 0))
          (bind _output_get (Variables|Default|SetWeapon _returnvalue))
          (Transformation|AttachComponentToComponent _output_get (Variables|Character|GetMesh) "SK_Sword" "SnapToTarget" "SnapToTarget" "SnapToTarget" true)
          (Variables|Default|SetisWieldingWeapon true))))))

(event EventBeginPlay
  (|CallParentFunction))

(event EventAttack
  (bind _returnvalue (Transformation|GetActorLocation))
  ;[0.15 0.15 0.15 0.5] Attack player
  (bind _notifyname (Animation|Montage|PlayMontage (Variables|Character|GetMesh) "/Game/ENEMY/animation/montage/Sword_And_Shield_Slash_Montage.Sword_And_Shield_Slash_Montage")
    (:then
      (Variables|/Game/Damage_System/BPC_DamageSystem.BPC_DamageSystem_C|SetIsInterruptible (Variables|Default|GetBPC_DamageSystem) false))
    (:OnCompleted
      (Default|CallOnAttackEnd :!label _label)
      (Variables|/Game/Damage_System/BPC_DamageSystem.BPC_DamageSystem_C|SetIsInterruptible (Variables|Default|GetBPC_DamageSystem) true))
    (:OnInterrupted
      (goto _label))
    (:OnNotifyBegin
      (switch name _notifyname
        (:Slash
          (bind _outhit (Collision|SphereTraceForObjects _returnvalue (+ _returnvalue (* (Transformation|GetActorForwardVector) 2e+02)) 2e+01 (Utilities|Array|MakeArray "ObjectTypeQuery3") false 0 "ForDuration"))
          (if true
            (bind _returnvalue_2 (Utilities|GetDataTableRow "/Game/ENEMY/DataTable/DT_DamagePower.DT_DamagePower" "Value")
              (:then
                (Class|BPIDamageable|TakeDamage(Message) (.HitActor (Collision|BreakHitResult _outhit)) (Utilities|Struct|MakeST_DamageInfo (.Sword (Utilities|Struct|BreakST_DamagePower _returnvalue_2)) "NewEnumerator1"))))))))))

(fn ConstructionScript
  (|CallParentFunction))