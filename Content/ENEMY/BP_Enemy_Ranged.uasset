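; Ranged enemy AI character that spawns a bow on begin play, attaches it to its mesh and fires arrows at its AI controller's attack target.
; Attack and reload are montage-driven: notifies fire through the BPCAttacks component or attach a loaded arrow, and montage end calls the attack-end or weapon-equipped events.
; It also maps movement states to walk speeds and reads attack and defend radii from a data table.
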(event Custom|ReloadBow
  ;[0.15 0.15 0.15 0.5] Load Arrow to bow
  (bind _notifyname (Animation|Montage|PlayMontage (Variables|Character|GetMesh) "/Game/ENEMY/animation/montage/Shooting_Arrow_Montage.Shooting_Arrow_Montage")
    (:OnCompleted
      (Default|CallOnWeaponEquiped :!label _label))
    (:OnInterrupted
      (goto _label))
    (:OnNotifyBegin
      (switch name _notifyname
        (:Spawn%20Arrow
          (bind _returnvalue (Game|SpawnActorfromClass "/Game/Weapons/BP_ArrowNONe.BP_ArrowNONe_C" (Transformation|GetActorTransform) "Undefined" "MultiplyWithRoot" 0 0))
          (bind _output_get (Variables|Default|SetSpawedArrow _returnvalue))
          (Transformation|AttachComponentToComponent _output_get (Variables|Character|GetMesh) "SK_Arrow" "SnapToTarget" "SnapToTarget" "SnapToTarget" true)
          (Variables|Default|SetHasLoadedArrow true))))))

(event EventBeginPlay
  ;[0.15 0.15 0.15 0.5] begin play to equip the bow to the AI
  (|CallParentFunction)
  (CallFunction|EquipWeapon))

(event EventEquipWeapon
  ;[0.15 0.15 0.15 0.5] Equip bow
  (bind _returnvalue (Game|SpawnActorfromClass "/Game/Weapons/BP_Bow.BP_Bow_C" (Math|Transform|MakeTransform "0, 0, 0") "Undefined" "MultiplyWithRoot" 0 0))
  (bind _output_get (Variables|Default|SetWeapon _returnvalue))
  (Transformation|AttachComponentToComponent _output_get (Variables|Character|GetMesh) "SK_Bow" "KeepRelative" "KeepRelative" "KeepRelative" true)
  (Variables|Default|SetisWieldingWeapon true)
  (Default|CallOnWeaponEquiped))

(event EventAttack
  ;[0.15 0.15 0.15 0.5] Attack Player
  (Variables|Default|SetAttacking true)
  (bind _notifyname (Animation|Montage|PlayMontage (Variables|Character|GetMesh) "/Game/ENEMY/animation/montage/Standing_Aim_Recoil_Montage.Standing_Aim_Recoil_Montage")
    (:OnCompleted
      (Default|CallOnAttackEnd :!label _label)
      (Variables|Default|SetHasLoadedArrow false)
      (Variables|Default|SetAttacking false))
    (:OnInterrupted
      (goto _label))
    (:OnNotifyBegin
      (switch name _notifyname
        (:Fire
          (bind _asaic_enemy_base (Utilities|Casting|CastToAIC_EnemyBase (AI|GetAIController self)))
          (bind _attack_target (Variables|/Game/ENEMY/AI/AIC_EnemyBase.AIC_EnemyBase_C|GetAttack%20Target _asaic_enemy_base)
            (:then
              (Default|Arrow (Variables|Default|GetBPC_Attacks) (Transformation|GetActorLocation (Variables|Default|GetWeapon)) (Transformation|GetActorLocation _attack_target) (Transformation|GetActorTransform) self))
            (:else)))))))

(fn ConstructionScript
  (|CallParentFunction))

(fn SetMoveSpeed
  (params (Speed :type E_MoveSpeed%20Enum :default "NewEnumerator0"))
  ;[0.15 0.15 0.15 0.5] set movement speed
  (bind _output_get (Variables|/Script/Engine.CharacterMovementComponent|SetMaxWalkSpeed (Variables|Character|GetCharacterMovement) (Utilities|Select :Index Speed :NewEnumerator0 0.0 :NewEnumerator1 2e+02 :NewEnumerator2 3e+02 :NewEnumerator3 5e+02)))
  (return _output_get))

(fn GetIdealRange
  ;[0.15 0.15 0.15 0.5] Attacking and defending distance
  (bind _returnvalue (Utilities|GetDataTableRow "/Game/ENEMY/DataTable/DT_AIMoveRadius.DT_AIMoveRadius" "Ranged_AI")
    (:then
      (return (.AttackRadius (Utilities|Struct|BreakST_AIMoveRadius _returnvalue)) (.DefendRadius (Utilities|Struct|BreakST_AIMoveRadius _returnvalue))))))