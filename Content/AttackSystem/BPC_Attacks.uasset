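; Attack component that performs a magic spell and a bow arrow attack for its owning actor.
; MagicSpell spawns a targeted BP_BlueEnergy projectile, applies the passed damage info on impact, then signals attack end.
; Arrow line-traces for a pawn, fires BP_Arrow at it, and applies DT_DamagePower bow damage only if that pawn is hit.
; Both attacks send damage through TakeDamageMessage and report it to AI damage sensing.
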(event Custom|MagicSpell
  (params (SpawnTransform :type Transform) (Target :type Actor%20Object%20Reference) (DamegeInfo :type ST%20Damage%20Info%20Structure))
  ;[0.15 0.15 0.15 0.5] Magic Spell and report damage
  (bind _returnvalue (Game|SpawnActorfromClass "/Game/Projectiles/BP_BlueEnergy.BP_BlueEnergy_C" SpawnTransform "Undefined" "MultiplyWithRoot" (Components|GetOwner) 1.5e+03 0.0 Target true 0))
  (EventDispatchers|BindEventtoOnProjectileImpact _returnvalue (delegate Custom|OnProjectileHit))
  (Collision|IgnoreActorwhenMoving (Variables|/Game/Projectiles/BP_Projecctile_Base.BP_Projecctile_Base_C|GetBox%20collision _returnvalue) (Game|GetPlayerCharacter 0) true))

(event Custom|OnProjectileHit
  (params (Other%20Actor :type Actor%20Object%20Reference) (Hit :type Hit%20Result%20Structure))
  ;[0.15 0.15 0.15 0.5] Magic Spell and report damage
  (Class|BPIDamageable|TakeDamage(Message) Other%20Actor (stale Custom|MagicSpell DamegeInfo) (Components|GetOwner))
  (Class|AISenseDamage|ReportDamageEvent Other%20Actor (Components|GetOwner) (.Amount (Utilities|Struct|BreakST_DamageInfo (stale Custom|MagicSpell DamegeInfo))) (Transformation|GetActorLocation (Components|GetOwner)) "0, 0, 0" "None")
  (Default|CallOnAttackEnded))

(event Custom|Arrow
  (params (Trace%20Start :type Vector) (Trace%20End :type Vector) (Arrow%20Transform :type Transform) (Actor :type Actor%20Object%20Reference))
  ;[0.15 0.15 0.15 0.5] Arrow Damage
  (bind (_outhit _returnvalue) (Collision|LineTraceForObjects Trace%20Start Trace%20End (Utilities|Array|MakeArray "ObjectTypeQuery3") false 0 "ForDuration"))
  (if _returnvalue
    (bind _returnvalue_2 (Game|SpawnActorfromClass "/Game/Projectiles/BP_Arrow.BP_Arrow_C" Arrow%20Transform "Undefined" "MultiplyWithRoot" (Components|GetOwner) 2e+03 0.0 (.HitActor (Collision|BreakHitResult _outhit)) false 0))
    (Collision|IgnoreActorwhenMoving (Variables|/Game/Projectiles/BP_Projecctile_Base.BP_Projecctile_Base_C|GetBox%20collision _returnvalue_2) (Components|GetOwner) true)
    (Collision|AssignOnActorHit _returnvalue_2 (delegate Custom|OnActorHit_Event))))

(event Custom|OnActorHit_Event
  (params (SelfActor :type Actor%20Object%20Reference) (OtherActor :type Actor%20Object%20Reference) (NormalImpulse :type Vector) (Hit :type Hit%20Result%20Structure%20%28by%20ref%29))
  (bind _returnvalue (Components|GetOwner))
  ;[0.15 0.15 0.15 0.5] Arrow Damage
  (if (== (.HitActor (Collision|BreakHitResult Hit)) (.HitActor (Collision|BreakHitResult (stale Custom|Arrow _outhit))))
    (bind _returnvalue_2 (Utilities|GetDataTableRow "/Game/ENEMY/DataTable/DT_DamagePower.DT_DamagePower" "Value")
      (:then
        (Class|BPIDamageable|TakeDamage(Message) (.HitActor (Collision|BreakHitResult (stale Custom|Arrow _outhit))) (Utilities|Struct|MakeST_DamageInfo (.Bow (Utilities|Struct|BreakST_DamagePower _returnvalue_2)) "NewEnumerator2" "NewEnumerator0" false true) _returnvalue)
        (Class|AISenseDamage|ReportDamageEvent (.HitActor (Collision|BreakHitResult (stale Custom|Arrow _outhit))) _returnvalue (.Bow (Utilities|Struct|BreakST_DamagePower _returnvalue_2)) (Transformation|GetActorLocation (Components|GetOwner)) "0, 0, 0" "None")))))